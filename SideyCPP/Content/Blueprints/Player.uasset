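; Player character Blueprint for a web-swinging game, handling camera look, grounded state, swing point scanning and wall hits.
; Each Tick updates Grounded from character movement, applies yaw to the controller and pitch to the camera, and checks capsule overlaps for SwingingCollision actors to call HitWall.
; FindSwingPoint gathers WebPoints overlapping PointDetection into the scanned list, clearing TryingToSwing when a cast fails.
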(event EventBeginPlay)

(event Collision|EventActorBeginOverlap
  (params (OtherActor :type Actor%20Object%20Reference)))

(event EventTick
  (params (DeltaSeconds :type Float%20%28single-precision%29))
  (CallFunction|GroundedCheck)
  (CallFunction|Rotation)
  (CallFunction|BuildingCheck))

(event EventFindSwingPoint
  (for _array_element (Collision|GetOverlappingActors (Variables|Default|GetPointDetection) "/Game/Blueprints/WebPoint_Base.WebPoint_Base_C" :!class /Script/Engine.PrimitiveComponent)
    (bind _asweb_point (Utilities|Casting|CastToWebPoint _array_element)
      (:then
        (Utilities|Array|Add (Variables|Default|GetScannedPoints) _asweb_point)
        (Class|PlayerBase|SetScannedObjects (Variables|Default|GetScannedPoints)))
      (:CastFailed
        (Development|PrintString "Failed To Cast Points")
        (Variables|Default|SettryingToSwing false)))))

(fn ConstructionScript)

(fn GroundedCheck
  (Variables|Default|Setgrounded (not (AI|Components|NavMovement|IsFalling (Variables|Character|GetCharacterMovement self)))))

(fn Rotation
  (bind _self self)
  (Pawn|Input|AddControllerYawInput (Variables|Default|GetyawChange _self))
  (Transformation|AddLocalRotation (Variables|Default|GetCamera) (Variables|Default|GetpitchChange _self) false false))

(fn BuildingCheck
  (for _array_element (Collision|GetOverlappingActors (Variables|Default|GetCapsuleComponent) 0 :!class /Script/Engine.PrimitiveComponent)
    (Utilities|Casting|CastToSwingingCollision _array_element)
    (Class|PlayerBase|HitWall self)
    (Development|PrintString "I hit something")))